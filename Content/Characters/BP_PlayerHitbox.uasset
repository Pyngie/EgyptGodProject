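; BP_PlayerHitbox is a short-lived player attack hitbox actor that damages enemies it touches and destroys itself half a second after spawning.
; Its capsule overlap applies the Damage value to BP_Enemy actors, naming the player pawn as damage causer.
; An AlreadyDamage list records each enemy hit, so every enemy takes damage only once per hitbox.
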(event OnComponentBeginOverlap(Capsule)
  (params (OverlappedComponent :type Primitive%20Component%20Object%20Reference) (OtherActor :type Actor%20Object%20Reference) (OtherComp :type Primitive%20Component%20Object%20Reference) (OtherBodyIndex :type Integer) (bFromSweep :type Boolean) (SweepResult :type Hit%20Result%20Structure%20%28by%20ref%29))
  (bind _asbp_enemy (Utilities|Casting|CastToBP_Enemy OtherActor))
  (if (not (Utilities|Array|ContainsItem (Variables|Default|GetAlreadyDamage) _asbp_enemy))
    (Utilities|Array|Add (Variables|Default|GetAlreadyDamage) _asbp_enemy)
    (Game|Damage|ApplyDamage OtherActor (Variables|Default|GetDamage) 0 (Game|Player|GetPlayerPawn 0))))

(event Collision|EventActorBeginOverlap
  (params (OtherActor :type Actor%20Object%20Reference)))

(event EventTick
  (params (DeltaSeconds :type Float%20%28single-precision%29)))

(event EventBeginPlay
  (Utilities|FlowControl|Delay 0.5)
  (Actor|DestroyActor))

(fn ConstructionScript)