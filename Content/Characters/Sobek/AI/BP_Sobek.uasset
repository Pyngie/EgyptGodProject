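; Sobek AI enemy character with light, medium and charged heavy attacks, plus a timed block.
; Tick feeds health percent and cooldown readiness to the Blackboard, counting medium and heavy only after a first light attack, and launches Sobek at its target while AimAtPlayer is set.
; Attack events play montages; separate functions spawn attached damage spheres.
; Damage is cut to a third while BlockTimeEnd is false, otherwise triggering stagger and knockback unless attacking.
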(event Custom|Blocking
  ;[0.15 0.15 0.15 0.5] Block
  (AI|Components|Blackboard|SetValueasBool (AI|GetBlackboard 0) (Utilities|Name|MakeLiteralName "inCombat") true)
  (Variables|Default|SetBlockCooldownTimer 0.0)
  (Animation|PlayAnimMontage "/Game/Characters/Sobek/Attack/BlockIdle_Montage.BlockIdle_Montage" 1.0 "None")
  (Utilities|FlowControl|Delay 3.3)
  (CallFunction|EndBlocking))

(event Custom|StartLightAttack
  (AI|Components|Blackboard|SetValueasBool (AI|GetBlackboard 0) (Utilities|Name|MakeLiteralName "inCombat") true)
  (Variables|Default|SetUnlockingAttack true)
  (Variables|Default|SetisAttacking true)
  (Animation|PlayAnimMontage "/Game/Characters/Sobek/Attack/Attack_Light_Montage.Attack_Light_Montage" 1.0 "None"))

(event Custom|StartMediumAttack
  (AI|Components|Blackboard|SetValueasBool (AI|GetBlackboard 0) (Utilities|Name|MakeLiteralName "inCombat") true)
  (Variables|Default|SetisAttacking true)
  (Variables|Default|SetMediumTimer 0.0)
  (bind _returnvalue (Animation|PlayAnimMontage "/Game/Characters/Sobek/Attack/Attack_Medium_Montage.Attack_Medium_Montage" 1.0 "None"))
  (Utilities|FlowControl|Delay _returnvalue)
  (Variables|Default|SetMediumEnd true)
  (AI|Components|Blackboard|SetValueasBool (AI|GetBlackboard 0) (Utilities|Name|MakeLiteralName "MediumAttackReady") false))

(event Custom|Blockingcooldown
  (if (not (ScalableFloat|GetValueasBool (AI|GetBlackboard 0) (Utilities|Name|MakeLiteralName "BlockReady")))
    (Variables|Default|SetBlockCooldownTimer (+ (Utilities|Time|GetWorldDeltaSeconds) (Variables|Default|GetBlockCooldownTimer)))
    (if (>= (Variables|Default|GetBlockCooldownTimer) (Variables|Default|GetBlockCooldown))
      (AI|Components|Blackboard|SetValueasBool (AI|GetBlackboard 0) (Utilities|Name|MakeLiteralName "BlockReady") true))))

(event Custom|MediumCooldown
  (if (not (ScalableFloat|GetValueasBool (AI|GetBlackboard 0) (Utilities|Name|MakeLiteralName "MediumAttackReady")))
    (Variables|Default|SetMediumTimer (+ (Utilities|Time|GetWorldDeltaSeconds) (Variables|Default|GetMediumTimer)))
    (if (>= (Variables|Default|GetMediumTimer) (Variables|Default|GetMediumTIme))
      (AI|Components|Blackboard|SetValueasBool (AI|GetBlackboard 0) (Utilities|Name|MakeLiteralName "MediumAttackReady") true))))

(event Custom|EndBlocking
  ;[0.15 0.15 0.15 0.5] Block
  (AI|Components|Blackboard|SetValueasBool (AI|GetBlackboard 0) (Utilities|Name|MakeLiteralName "BlockReady") false)
  (AI|Components|Blackboard|SetValueasBool (AI|GetBlackboard 0) (Utilities|Name|MakeLiteralName "inCombat") false)
  (Variables|Default|SetBlockTimeEnd true))

(event Custom|StartHeavyAttack
  (AI|Components|Blackboard|SetValueasBool (AI|GetBlackboard 0) (Utilities|Name|MakeLiteralName "inCombat") true)
  (Variables|Default|SetTargetActor (Game|GetPlayerCharacter 0))
  (Variables|Default|SetisAttacking true)
  (Variables|Default|SetHeavyTImer 0.0)
  (Animation|Montage|PlayMontage (Variables|Character|GetMesh) "/Game/Characters/Sobek/Attack/Attack_HeavyCharge_Montage.Attack_HeavyCharge_Montage"
    (:OnCompleted
      (Animation|Montage|PlayMontage (Variables|Character|GetMesh) "/Game/Characters/Sobek/Attack/Attack_Heavy_Montage1.Attack_Heavy_Montage1"
        (:OnCompleted
          (Variables|Default|SetHeavyEnd true)
          (AI|Components|Blackboard|SetValueasBool (AI|GetBlackboard 0) (Utilities|Name|MakeLiteralName "HeavyAttackReady") false))))))

(event Custom|HeavyCooldown
  (if (not (ScalableFloat|GetValueasBool (AI|GetBlackboard 0) (Utilities|Name|MakeLiteralName "HeavyAttackReady")))
    (Variables|Default|SetHeavyTImer (+ (Utilities|Time|GetWorldDeltaSeconds) (Variables|Default|GetHeavyTImer)))
    (if (>= (Variables|Default|GetHeavyTImer) (Variables|Default|GetHeavyTime))
      (AI|Components|Blackboard|SetValueasBool (AI|GetBlackboard 0) (Utilities|Name|MakeLiteralName "HeavyAttackReady") true))))

(event EventBeginPlay
  (|CallParentFunction) ; This node is disabled and will not be called.\nDrag off pins to build functionality.
)

(event Collision|EventActorBeginOverlap
  (params (OtherActor :type Actor%20Object%20Reference)))

(event EventTick
  (params (DeltaSeconds :type Float%20%28single-precision%29))
  (bind _returnvalue (Transformation|GetActorLocation))
  (bind _targetactor (Variables|Default|GetTargetActor))
  (bind _returnvalue_2 (Transformation|GetActorLocation _targetactor))
  (bind _returnvalue_3 (- _returnvalue_2 _returnvalue))
  (bind (_x _y) (Math|Vector|BreakVector _returnvalue_3))
  (|CallParentFunction DeltaSeconds)
  (AI|Components|Blackboard|SetValueasFloat (AI|GetBlackboard 0) (Utilities|Name|MakeLiteralName "HealthPercent") (* (/ (Variables|Default|GetCurrentHealth) (Variables|Default|GetMaxHealth)) 1e+02))
  (CallFunction|Blockingcooldown)
  (if (Variables|Default|GetUnlockingAttack)
    (CallFunction|MediumCooldown)
    (CallFunction|HeavyCooldown))
  (if (Variables|Default|GetAimAtPlayer)
    (Character|LaunchCharacter (* (Math|Vector|Normalize (Math|Vector|MakeVector _x _y 0.0)) 6e+02) true false)))

(event EventBeginPlay
  (Variables|Default|SetMaxHealth 3.5e+02)
  (Variables|Default|SetCurrentHealth (Variables|Default|GetMaxHealth)))

(event EventAnyDamage
  (params (Damage :type Float%20%28single-precision%29) (DamageType :type Damage%20Type%20Object%20Reference) (InstigatedBy :type Controller%20Object%20Reference) (DamageCauser :type Actor%20Object%20Reference))
  (if (and (not (Variables|Default|GetisDead)) (not (Variables|Default|GetisHurt)))
    (if (Variables|Default|GetBlockTimeEnd)
      (Variables|Default|SetCurrentHealth (Math|Float|Clamp(Float) (- (Variables|Default|GetCurrentHealth) Damage) 0.0 (Variables|Default|GetMaxHealth)))
      (if (not (Variables|Default|GetisAttacking))
        (if (Variables|Default|GetgotStun)
          (Variables|Default|SetisHurt true)
          (Animation|PlayAnimMontage "/Game/Characters/Sobek/Hurt/Hurt_Montage.Hurt_Montage" 1.0 "None")
          (else
            (Variables|Default|SetisHurt true)
            (Animation|PlayAnimMontage "/Game/Characters/Sobek/Hurt/Hurt_Montage.Hurt_Montage" 1.0 "None")))
        (Character|LaunchCharacter (* (Math|Vector|Normalize (- (Transformation|GetActorLocation) (Transformation|GetActorLocation DamageCauser))) 3e+02) true false)
        (CallFunction|Stun)
        (Variables|Default|SetgotStun false)
        (Utilities|FlowControl|Delay 0.4)
        (Variables|Default|SetisHurt false))
      (else
        ;[0.15 0.15 0.15 0.5] Less Damage when Block
        (Variables|Default|SetCurrentHealth (Math|Float|Clamp(Float) (- (Variables|Default|GetCurrentHealth) (/ Damage 3.0)) 0.0 (Variables|Default|GetMaxHealth)))
        (Variables|Default|SetisHurt true)
        (Utilities|FlowControl|Delay 0.4)
        (Variables|Default|SetisHurt false)))))

(fn ConstructionScript
  (|CallParentFunction))

(fn SpawnLightAttack
  (bind _returnvalue (Game|SpawnActorfromClass "/Game/Characters/Sobek/AI/LightAttackSphere.LightAttackSphere_C" (Math|Conversions|ToTransform(Vector) (+ (Transformation|GetWorldLocation (Variables|Character|GetMesh)) (* (Transformation|GetActorForwardVector self) 95.0) "0.000000,0.000000,150.000000")) "Undefined" "MultiplyWithRoot" 0 15.0 0))
  (Transformation|AttachActorToActor _returnvalue self "None" "SnapToTarget" "SnapToTarget" "KeepWorld" false))

(fn SpawnMediumAttack
  (bind _returnvalue (Game|SpawnActorfromClass "/Game/Characters/Sobek/AI/MediumAttackSphere.MediumAttackSphere_C" (Math|Conversions|ToTransform(Vector) (+ (Transformation|GetWorldLocation (Variables|Character|GetMesh)) (* (Transformation|GetActorForwardVector self) 95.0) "0.000000,0.000000,150.000000")) "Undefined" "MultiplyWithRoot" 0 25.0 0))
  (Transformation|AttachActorToActor _returnvalue self "None" "SnapToTarget" "SnapToTarget" "KeepWorld" false))

(fn SpawnHeavyAttack
  (bind _returnvalue (Game|SpawnActorfromClass "/Game/Characters/Sobek/AI/HeavyAttackSphere.HeavyAttackSphere_C" (Math|Conversions|ToTransform(Vector) (+ (Transformation|GetWorldLocation (Variables|Character|GetMesh)) (* (Transformation|GetActorForwardVector self) 95.0) "0.000000,0.000000,150.000000")) "Undefined" "MultiplyWithRoot" 0 6e+01 0))
  (Transformation|AttachActorToActor _returnvalue self "None" "SnapToTarget" "SnapToTarget" "KeepWorld" false))