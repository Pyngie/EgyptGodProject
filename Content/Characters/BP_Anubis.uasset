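; BP_Anubis is a character Blueprint for Anubis that handles its reaction to taking damage.
; AnyDamage, ignored while dead or hurt, reduces clamped health, plays a hit montage and knocks the character away from the damage causer.
; It then calls Stun, clears GotStun and lifts the hurt lockout after a short delay.
; Both GotStun branches are identical, and no death logic appears here.
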(event EventBeginPlay
  (|CallParentFunction) ; This node is disabled and will not be called.\nDrag off pins to build functionality.
)

(event Collision|EventActorBeginOverlap
  (params (OtherActor :type Actor%20Object%20Reference)))

(event EventTick
  (params (DeltaSeconds :type Float%20%28single-precision%29))
  (|CallParentFunction DeltaSeconds) ; This node is disabled and will not be called.\nDrag off pins to build functionality.
)

(event EventAnyDamage
  (params (Damage :type Float%20%28single-precision%29) (DamageType :type Damage%20Type%20Object%20Reference) (InstigatedBy :type Controller%20Object%20Reference) (DamageCauser :type Actor%20Object%20Reference))
  (if (and (not (Variables|Default|GetisDead)) (not (Variables|Default|GetisHurt)))
    (Variables|Default|SetCurrentHealth (Math|Float|Clamp(Float) (- (Variables|Default|GetCurrentHealth) Damage) 0.0 2e+02))
    (if (Variables|Default|GetgotStun)
      (Variables|Default|SetisHurt true)
      (Animation|PlayAnimMontage "/Game/Characters/Anubis/Hurt/Hit_Montage.Hit_Montage" 1.0 "None")
      (else
        (Variables|Default|SetisHurt true)
        (Animation|PlayAnimMontage "/Game/Characters/Anubis/Hurt/Hit_Montage.Hit_Montage" 1.0 "None")))
    (Character|LaunchCharacter (* (Math|Vector|Normalize (- (Transformation|GetActorLocation) (Transformation|GetActorLocation DamageCauser))) 6e+02) true false)
    (CallFunction|Stun)
    (Variables|Default|SetgotStun false)
    (Utilities|FlowControl|Delay 0.4)
    (Variables|Default|SetisHurt false)))

(fn ConstructionScript
  (|CallParentFunction))